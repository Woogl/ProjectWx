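; PCG Blueprint element that filters point data down to points whose referenced actor has collision enabled, housed with the Forest PCG modules.
; The point loop resolves each point's ActorReference soft path attribute to an actor and tests collision on its root component.
; Points are dropped when the actor does not resolve, its root is not a primitive component, or collision is disabled.
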(fn PointLoopBody
  (params (InPointData :type PCG%20Base%20Point%20Data%20Object%20Reference) (InPoint :type PCG%20Point%20Structure%20%28by%20ref%29) (OutPointData :type PCG%20Base%20Point%20Data%20Object%20Reference) (PointIndex :type Integer64))
  (bind _returnvalue (Class|PCGMetadataAccessorHelpers|GetSoftObjectPathAttribute InPoint (Metadata|ConstMetadata InPointData) "ActorReference"))
  (bind _asactor (Utilities|Casting|CastToActor (Utilities|ResolveSoftReference (Class|KismetSystemLibrary|ToSoftObjRef(SoftObjPath) _returnvalue)))
    (:then
      (bind _asprimitive_component (Utilities|Casting|CastToPrimitiveComponent (Variables|/Script/Engine.Actor|GetRootComponent _asactor))
        (:then
          (return InPoint (Class|PrimitiveComponent|IsCollisionEnabled _asprimitive_component)))
        (:CastFailed
          (return InPoint false))))
    (:CastFailed
      (return InPoint false))))